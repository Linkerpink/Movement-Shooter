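; BP_EnemyBase is an enemy pawn that chases the player on sight and ragdolls or tumbles physically when killed.
; Pawn sensing triggers an AI move toward the first player's character, stopping within an acceptance radius.
; Damage reduces health initialized from its maximum; at zero, the mesh simulates physics and receives an impulse along the player's first-person camera direction.
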(event OnSeePawn(PawnSensing)
  (params (Pawn :type Pawn%20Object%20Reference))
  (CallFunction|ChasePlayer))

(event Custom|TakeDamage
  (params (DamageAmount :type Float%20%28double-precision%29))
  (Variables|Default|SetHp (- (Variables|Default|GetHp) DamageAmount))
  (if (<= (Variables|Default|GetHp) 0)
    (CallFunction|Die)))

(event Custom|Die
  (bind _mesh (Variables|Character|GetMesh))
  (Physics|SetSimulatePhysics _mesh true)
  (bind _asbp_player (Utilities|Casting|CastToBP_Player (Game|Player|GetPlayerPawn 0)))
  (Physics|AddImpulse _mesh (* (Math|Vector|GetForwardVector (Variables|/Game/Blueprints/BP_Player.BP_Player_C|GetFirstPersonCamera _asbp_player)) "25.000000,25.000000,25.000000") "None" false))

(event Custom|Chase%20Player
  (AI|AIMoveTo self "0, 0, 0" (Game|GetPlayerCharacter 0) 1.2e+02 false))

(event EventBeginPlay
  (Variables|Default|SetHp (Variables|Default|GetMaxHp)))

(fn ConstructionScript)