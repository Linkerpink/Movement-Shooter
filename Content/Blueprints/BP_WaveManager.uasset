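; Wave manager that runs endless, escalating enemy waves, starting at BeginPlay.
; NewWave increments and prints the wave number, then spawns that many BP_EnemyBase actors, each at a randomly picked spawn point transform.
; RemoveEnemyFromWave decrements the remaining count and starts the next wave when it reaches zero.
; RandomInteger(3) yields only 0–2, so SpawnPoint4 is never selected.
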(event Custom|NewWave
  ;[0.15 0.15 0.15 0.5] New Wave
  (Variables|Default|SetWave (+ (Variables|Default|GetWave) 1))
  (Development|PrintString (Utilities|String|ToString(Integer) (Variables|Default|GetWave)) true true "(R=1.000000,G=0.000000,B=0.000000,A=1.000000)")
  (for _index (range 1 (Variables|Default|GetWave))
    (Variables|Default|SetEnemiesLeftInWave (+ (Variables|Default|GetEnemiesLeftInWave) 1))
    (CallFunction|GetRandomSpawn)
    (Game|SpawnActorfromClass "/Game/Blueprints/BP_EnemyBase.BP_EnemyBase_C" (Variables|Default|GetRND%20Spawn%20Location) "Undefined" "MultiplyWithRoot" 0 0)))

(event Custom|Remove%20Enemy%20From%20Wave
  ;[0.15 0.15 0.15 0.5] Remove Enemy From Wave'
  (Variables|Default|SetEnemiesLeftInWave (- (Variables|Default|GetEnemiesLeftInWave) 1))
  (if (<= (Variables|Default|GetEnemiesLeftInWave) 0)
    (CallFunction|NewWave)))

(event Custom|Get%20Random%20Spawn
  ;[0.15 0.15 0.15 0.5] Get Random Spawn
  (bind _output_get (Variables|Default|SetRND (Math|Random|RandomInteger 3)))
  (switch int _output_get
    (:0
      (Variables|Default|SetRND%20Spawn%20Location (Transformation|GetWorldTransform (Variables|Default|GetSpawnPoint1))))
    (:1
      (Variables|Default|SetRND%20Spawn%20Location (Transformation|GetWorldTransform (Variables|Default|GetSpawnPoint2))))
    (:2
      (Variables|Default|SetRND%20Spawn%20Location (Transformation|GetWorldTransform (Variables|Default|GetSpawnPoint3))))
    (:3
      (Variables|Default|SetRND%20Spawn%20Location (Transformation|GetWorldTransform (Variables|Default|GetSpawnPoint4))))))

(event EventBeginPlay
  (CallFunction|NewWave))

(fn ConstructionScript)