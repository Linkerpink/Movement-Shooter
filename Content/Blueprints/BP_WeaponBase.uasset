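; Base weapon Blueprint that handles hitscan shooting, magazine-based ammo and its on-screen HUD.
; BeginPlay creates WBP_HUD and calls Reload, which spends a magazine, refills Ammo and refreshes the HUD.
; Shoot, limited by a Tick-driven cooldown, line-traces from the player camera, damages BP_EnemyBase hits found by display-name match, and auto-reloads on empty.
; The reload timer counts down but does not gate shooting here.
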(event Custom|Update%20Ammo%20UI
  ;[0.15 0.15 0.15 0.5] Update Ammo UI
  (Rendering|Components|TextRender|SetText (Variables|/Game/Widgets/WBP_HUD.WBP_HUD_C|GetAmmoText (Variables|Default|GetHud%20Widget)) (Utilities|Text|FormatText "Ammo: {Amount} / {MagSize}" (Variables|Default|GetAmmo) (Variables|Default|GetMagSize))))

(event Custom|Update%20Mags%20UI
  ;[0.15 0.15 0.15 0.5] Update Mags UI
  (Rendering|Components|TextRender|SetText (Variables|/Game/Widgets/WBP_HUD.WBP_HUD_C|GetMagsText (Variables|Default|GetHud%20Widget)) (Utilities|Text|FormatText "Mags: {Amount}" (Variables|Default|GetMags))))

(event EventTick
  (params (DeltaSeconds :type Float%20%28single-precision%29))
  ;[0.15 0.15 0.15 0.5] Timers
  (Utilities|FlowControl|Sequence
    (:then_0
      (if (> (Variables|Default|GetShootTimer) 0.0)
        (Variables|Default|SetShootTimer (- (Variables|Default|GetShootTimer) DeltaSeconds))))
    (:then_1
      (if (> (Variables|Default|GetReloadTimer) 0.0)
        (Variables|Default|SetReloadTimer (- (Variables|Default|GetReloadTimer) DeltaSeconds))))))

(event EventBeginPlay
  ;[0.15 0.15 0.15 0.5] Initialize
  (Utilities|FlowControl|Sequence
    (:then_0
      (bind _returnvalue (UserInterface|CreateWidget "/Game/Widgets/WBP_HUD.WBP_HUD_C"))
      (bind _output_get (Variables|Default|SetHud%20Widget _returnvalue))
      (UserInterface|Viewport|AddtoViewport _output_get 0))
    (:then_1
      (CallFunction|Reload))))

(fn ConstructionScript)

(fn Reload
  (if (> (Variables|Default|GetMags) 0)
    (Variables|Default|SetReloadTimer (Variables|Default|GetReloadTimerLength))
    (Variables|Default|SetMags (- (Variables|Default|GetMags) 1))
    (Variables|Default|SetAmmo (Variables|Default|GetMagSize))
    (CallFunction|UpdateAmmoUI)
    (CallFunction|UpdateMagsUI)
    (else
      (Development|PrintString "Not Enough Mags"))))

(fn Shoot
  (if (> (Variables|Default|GetAmmo) 0)
    (if (<= (Variables|Default|GetShootTimer) 0.0)
      (Utilities|FlowControl|Sequence
        (:then_0
          (Variables|Default|SetShootTimer (Variables|Default|GetShootTimerLength)))
        (:then_1
          (Variables|Default|SetAmmo (- (Variables|Default|GetAmmo) 1))
          (CallFunction|UpdateAmmoUI)
          (if (<= (Variables|Default|GetAmmo) 0)
            (CallFunction|Reload)))
        (:then_2
          (bind _asbp_player (Utilities|Casting|CastToBP_Player (Game|Player|GetPlayerPawn 0)))
          (bind _outhit (Collision|LineTraceForObjects (Transformation|GetWorldLocation (Variables|/Game/Blueprints/BP_Player.BP_Player_C|GetFirstPersonCamera _asbp_player)) (+ (Transformation|GetWorldLocation (Variables|/Game/Blueprints/BP_Player.BP_Player_C|GetFirstPersonCamera _asbp_player)) (* (Math|Vector|GetForwardVector (Variables|/Game/Blueprints/BP_Player.BP_Player_C|GetFirstPersonCamera _asbp_player)) (Variables|Default|GetRange))) (Variables|Default|GetObject%20Types) false (Utilities|Array|MakeArray (Game|GetPlayerCharacter 0)) "None"))
          (if (Utilities|String|Contains (Utilities|GetDisplayName (.HitActor (Collision|BreakHitResult _outhit))) "BP_EnemyBase")
            (bind _asbp_enemy_base (Utilities|Casting|CastToBP_EnemyBase (.HitActor (Collision|BreakHitResult _outhit))))
            (Default|TakeDamage _asbp_enemy_base (Variables|Default|GetDamage))
            (else
              (Development|PrintString "geen teo"))))))
    (else
      (CallFunction|Reload))))